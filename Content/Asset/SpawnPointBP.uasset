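; SpawnPointBP is a spawn point actor that periodically launches IceBall actors during play.
; Each tick it looks up the Global actor and, unless the game has ended or is paused, accumulates a timer.
; Roughly every three seconds it spawns a scaled-down IceBall at its own transform, applies a velocity-change impulse along its forward vector, and resets the timer.
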(event EventBeginPlay)

(event Collision|EventActorBeginOverlap
  (params (OtherActor :type Actor%20Object%20Reference)))

(event EventTick
  (params (DeltaSeconds :type Float%20%28single-precision%29))
  (bind _returnvalue (Transformation|GetActorTransform))
  (bind (_location _rotation) (Math|Transform|BreakTransform _returnvalue))
  (bind _outactors (Actor|GetAllActorsOfClass "/Game/Asset/Global.Global_C"))
  (if (not (or (Variables|/Game/Asset/Global.Global_C|GetGameEnds (Utilities|Array|Get(acopy) _outactors)) (Variables|/Game/Asset/Global.Global_C|GetGamePause (Utilities|Array|Get(acopy) _outactors))))
    (bind _output_get (Variables|Default|SetSpawnTimer (+ DeltaSeconds (Variables|Default|GetSpawnTimer))))
    (if (> _output_get 3.0)
      (bind _returnvalue_2 (Game|SpawnActorfromClass "/Game/Asset/IceBall.IceBall_C" (Math|Transform|MakeTransform _location _rotation "0.150000,0.150000,0.150000") "Undefined" 0 0))
      (Physics|AddImpulse (Variables|/Game/Asset/IceBall.IceBall_C|GetBall _returnvalue_2) (* (Transformation|GetActorForwardVector) 1e+02) "None" true)
      (Variables|Default|SetSpawnTimer 0.0))))

(fn ConstructionScript)